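; BP_Music is an actor that plays the game's background music through an Audio component.
; On BeginPlay it starts the main menu cue when IsMainMenu is set, otherwise a waiting drum filler cue.
; A ChangeMusic event swaps the sound to a random entry from the MusicSamples array and plays it from the start.
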(event Custom|ChangeMusic
  (Audio|Components|Audio|SetSound (Variables|Default|GetAudio) (.OutItem (Utilities|Array|Random (Variables|Default|GetMusicSamples))))
  (Audio|Components|Audio|Play (Variables|Default|GetAudio) 0.0))

(event EventBeginPlay
  (if (Variables|Default|GetIsMainMenu)
    (Audio|Components|Audio|SetSound (Variables|Default|GetAudio) "/Game/Audio/Music/MainMenu_v1_Cue.MainMenu_v1_Cue")
    (Audio|Components|Audio|Play (Variables|Default|GetAudio) 0.0)
    (else
      (Audio|Components|Audio|SetSound (Variables|Default|GetAudio) "/Game/Audio/Music/PoG_Drums_Waiting_Filler_Cue.PoG_Drums_Waiting_Filler_Cue")
      (Audio|Components|Audio|Play (Variables|Default|GetAudio) 0.0))))

(event Collision|EventActorBeginOverlap
  (params (OtherActor :type Actor%20Object%20Reference)))

(event EventTick
  (params (DeltaSeconds :type Float%20%28single-precision%29)))

(fn ConstructionScript)