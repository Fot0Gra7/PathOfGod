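; Behavior tree service that keeps an AI pawn's distance to its target current on the blackboard.
; On each AI tick it reads the "Target" blackboard object and casts it to BP_Player_Keco.
; It writes the pawn's distance to that player into the "DistanceToTarget" key, skipping the update when the pawn, target or cast is invalid.
; A debug print of the panther-to-player distance is left disconnected.
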(event EventReceiveTickAI
  (params (OwnerController :type AI%20Controller%20Object%20Reference) (ControlledPawn :type Pawn%20Object%20Reference) (DeltaSeconds :type Float%20%28single-precision%29))
  (bind _returnvalue (AI|GetBlackboard ControlledPawn))
  (bind _returnvalue_2 (Utilities|Name|MakeLiteralName "Target"))
  (bind _returnvalue_3 (AI|Components|Blackboard|GetValueasObject _returnvalue _returnvalue_2))
  (Utilities|IsValid ControlledPawn
    (:Is%20Valid
      (Utilities|IsValid _returnvalue_3
        (:Is%20Valid
          (bind _asbp_player_keco (Utilities|Casting|CastToBP_Player_Keco _returnvalue_3))
          (AI|Components|Blackboard|SetValueasFloat _returnvalue (Utilities|Name|MakeLiteralName "DistanceToTarget") (Transformation|GetDistanceTo ControlledPawn _asbp_player_keco)))))))