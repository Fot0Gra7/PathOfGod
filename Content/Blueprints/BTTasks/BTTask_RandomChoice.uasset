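; Behavior tree task that randomly picks one of two special attack choices for an AI.
; On execute, it rolls a random float against the SuccsessChanceIntIsZero variable and writes 0 to the SpecialAttackChoice blackboard int when the roll is lower, otherwise 1.
; The key name is hardcoded rather than exposed as a selector, and the task finishes successfully on either outcome.
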(event EventReceiveExecuteAI
  (params (OwnerController :type AI%20Controller%20Object%20Reference) (ControlledPawn :type Pawn%20Object%20Reference))
  (if (< (Math|Random|RandomFloatinRange 0.0 1.0) (Variables|Default|GetSuccsessChance%28IntIsZero%29))
    (Class|BlackboardComponent|SetValueasInt (AI|GetBlackboard ControlledPawn) (Utilities|Name|MakeLiteralName "SpecialAttackChoice"))
    (AI|BehaviorTree|FinishExecute true)
    (else
      (Class|BlackboardComponent|SetValueasInt (AI|GetBlackboard ControlledPawn) (Utilities|Name|MakeLiteralName "SpecialAttackChoice") 1)
      (AI|BehaviorTree|FinishExecute true))))