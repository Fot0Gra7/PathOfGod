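; Behavior Tree task that triggers a Pog enemy's special attack and fails if the pawn is already attacking.
; It calls SpecialAttack, clears the CanDoSpecialAttack flag set by the random-choice task, and raises blackboard flags for in-progress and cooldown states.
; It starts the pawn's cooldown timer, which later clears the cooldown flag, and finishes immediately without waiting for the animation.
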(event EventReceiveExecuteAI
  (params (OwnerController :type AI%20Controller%20Object%20Reference) (ControlledPawn :type Pawn%20Object%20Reference))
  (bind _asbp_pog_enemy_base (Utilities|Casting|CastToBP_Pog_Enemy_BASE ControlledPawn))
  (if (not (Variables|/Game/Blueprints/Characters/BP_Pog_Character_BASE.BP_Pog_Character_BASE_C|GetIsAttacking _asbp_pog_enemy_base))
    (Default|SpecialAttack _asbp_pog_enemy_base)
    ;[0 0.005208 0.002608 1 13] Обнуляем переменную, установленную таском рандомного выбора
    (AI|Components|Blackboard|SetValueasBool (AI|GetBlackboard _asbp_pog_enemy_base) (Utilities|Name|MakeLiteralName "CanDoSpecialAttack") false)
    ;[0 0.01042 0.006902 1 14] BB переменная, которая сбрасывается в конце анимации атаки
    (AI|Components|Blackboard|SetValueasBool (AI|GetBlackboard _asbp_pog_enemy_base) (Utilities|Name|MakeLiteralName "IsInSpecialAttack") true)
    ;[0 0.01042 0.007022] Включаем таймер в Pawn'е врага и устанавливаем Blackboard переменную в True, которую этот таймер позже переведёт обратно в False
    (AI|Components|Blackboard|SetValueasBool (AI|GetBlackboard _asbp_pog_enemy_base) (Utilities|Name|MakeLiteralName "IsSpecialAttackOnCD") true)
    (Default|StartSpecialAttackCooldownTimer _asbp_pog_enemy_base)
    (AI|BehaviorTree|FinishExecute true)
    (else
      (AI|BehaviorTree|FinishExecute false))))