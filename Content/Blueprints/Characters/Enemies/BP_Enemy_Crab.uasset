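; Crab enemy Blueprint for a flipbook-animated character that walks along its facing direction and turns at walls and ledges.
; WalkForward feeds movement input, while overlap events on the wall and ledge detectors call TurnCharacter.
; Tick picks the walk or idle flipbook from velocity.
; Footsteps play without animation notifies, by polling the walk flipbook's current frame, with a DoOnce preventing repeats within a frame.
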(event OnComponentBeginOverlap(WallDetector)
  (params (OverlappedComponent :type Primitive%20Component%20Object%20Reference) (OtherActor :type Actor%20Object%20Reference) (OtherComp :type Primitive%20Component%20Object%20Reference) (OtherBodyIndex :type Integer) (bFromSweep :type Boolean) (SweepResult :type Hit%20Result%20Structure%20%28by%20ref%29))
  (CallFunction|TurnCharacter))

(event OnComponentEndOverlap(LedgeDetector)
  (params (OverlappedComponent :type Primitive%20Component%20Object%20Reference) (OtherActor :type Actor%20Object%20Reference) (OtherComp :type Primitive%20Component%20Object%20Reference) (OtherBodyIndex :type Integer))
  (CallFunction|TurnCharacter))

(event Custom|WalkForward
  (params (ScaleValue :type Float%20%28single-precision%29))
  (Pawn|Input|AddMovementInput (Transformation|GetActorForwardVector) ScaleValue false))

(event EventBeginPlay
  (|CallParentFunction) ; This node is disabled and will not be called.\nDrag off pins to build functionality.
)

(event Collision|EventActorBeginOverlap
  (params (OtherActor :type Actor%20Object%20Reference))
  (|CallParentFunction OtherActor) ; This node is disabled and will not be called.\nDrag off pins to build functionality.
)

(event EventTick
  (params (DeltaSeconds :type Float%20%28single-precision%29))
  (bind _sprite (Variables|Default|GetSprite))
  (bind _returnvalue (Class|PaperFlipbookComponent|GetPlaybackPositioninFrames _sprite))
  (|CallParentFunction DeltaSeconds)
  (CallFunction|UpdateAnim)
  ;[0 0.04868 0.06771] Проигрываем звук без PaperZD и Paper2D
  (if (== (Class|PaperFlipbookComponent|GetFlipbook (Variables|Default|GetSprite)) "/Game/PaperAssets/Characters/Enemies/crab/crab__Walk.crab__Walk")
    (if (or (== _returnvalue 2) (== _returnvalue 4))
      (Utilities|FlowControl|DoOnce false :!label _label
        (:Completed
          (Audio|PlaySoundatLocation "/Game/Audio/SFX/Footstep_Crab_Cue.Footstep_Crab_Cue" (Transformation|GetActorLocation) "0, 0, 0" 1.0 1.0 0.0 0 0 0 0)))
      (else
        (goto _label Reset)))))

(fn ConstructionScript
  (|CallParentFunction))

(fn UpdateAnim
  (Sprite|SetFlipbook (Variables|Default|GetSprite) (select (> (Math|Vector|VectorLength (Transformation|GetVelocity)) 0.0) "/Game/PaperAssets/Characters/Enemies/crab/crab__Walk.crab__Walk" "/Game/PaperAssets/Characters/Enemies/crab/crab__Idle.crab__Idle")))