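; Base enemy character for side-on combat, driven by AI through Blackboard keys, that reports its defeat to the quest manager and spawns destruction VFX.
; Regular and special attacks lock movement and jump to animation nodes, with a special-attack cooldown timer.
; Gap jumps launch along a computed projectile arc, and landing restores movement and resumes smart-link path following.
; Tick syncs falling state and hops stuck enemies toward the player.
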(event Custom|OnDefeated
  (bind _outactors (Actor|GetAllActorsOfClass "/Game/Blueprints/Props/BP_QuestManager.BP_QuestManager_C"))
  (Utilities|IsValid (Utilities|Array|Get(acopy) _outactors)
    (:Is%20Valid
      (Default|RegisterEnemyKilled (Utilities|Array|Get(acopy) _outactors) (Variables|Default|GetEnemyType)))
    (:Is%20Not%20Valid
      _))
  (Actor|DestroyActor))

(event EventBeginPlay
  (|CallParentFunction)
  (EventDispatchers|BindEventtoDefeated (delegate Custom|OnDefeated)))

(event Collision|EventActorBeginOverlap
  (params (OtherActor :type Actor%20Object%20Reference))
  (|CallParentFunction OtherActor) ; This node is disabled and will not be called.\nDrag off pins to build functionality.
)

(event EventTick
  (params (DeltaSeconds :type Float%20%28single-precision%29))
  (|CallParentFunction DeltaSeconds)
  (Utilities|FlowControl|Sequence
    (:then_0
      (if (AI|Components|NavMovement|IsFalling (Variables|Character|GetCharacterMovement))
        (AI|Components|Blackboard|SetValueasBool (AI|GetBlackboard 0) (Utilities|Name|MakeLiteralName "IsFalling") true)
        (else
          (AI|Components|Blackboard|SetValueasBool (AI|GetBlackboard 0) (Utilities|Name|MakeLiteralName "IsFalling") false))))
    (:then_1
      (CallFunction|EnemyStuckCheck DeltaSeconds))))

(event EventDestroyed
  ;[0.07665 0.15 0 0.5] SpawnVFX
  (Game|SpawnActorfromClass "/Game/Blueprints/VFX/BP_VFX_EnemyDestroyed.BP_VFX_EnemyDestroyed_C" (Math|Transform|MakeTransform (Transformation|GetActorLocation) (Transformation|GetActorRotation) "1.000000,1.000000,1.000000") "Undefined" "MultiplyWithRoot" 0 0))

(event EventOnLanded
  (params (Hit :type Hit%20Result%20Structure%20%28by%20ref%29))
  (Utilities|FlowControl|Sequence
    (:then_0
      (if (and (not (Variables|Default|GetIsStunned)) (not (Variables|Default|GetIsAttacking)))
        (AI|Components|Blackboard|SetValueasBool (AI|GetBlackboard 0) (Utilities|Name|MakeLiteralName "CanMove") true)
        (Variables|Default|SetCanMove true)))
    (:then_1
      ;[0.15 0.15 0.15 0.5 16] Продолжение движения по маршруту, если ИИ прыгнул со SmartLink'a
      (Utilities|IsValid (Variables|Default|GetCurrentSmartLink)
        (:Is%20Valid
          (Class|NavLinkProxy|ResumePathFollowing (Variables|Default|GetCurrentSmartLink) self))))
    (:then_2
      (Variables|Default|SetJumpAnimEnded true)
      (Variables|Default|SetIsInJumpAnim false))))

(fn ConstructionScript
  (|CallParentFunction))

(fn RegularAttack
  (if (not (Variables|Default|GetIsStunned))
    (Variables|Default|SetIsAttacking true)
    (Variables|Default|SetCanMove false)
    (AI|Components|Blackboard|SetValueasBool (AI|GetBlackboard 0) (Utilities|Name|MakeLiteralName "CanMove") false)
    (Class|PaperZDAnimInstance|JumptoNode (Class|PaperZDCharacter|GetAnimInstance) "JumpRegularAttack" "None")))

(fn SpecialAttack
  (if (not (Variables|Default|GetIsStunned))
    (Variables|Default|SetIsAttacking true)
    (Variables|Default|SetCanMove false)
    (AI|Components|Blackboard|SetValueasBool (AI|GetBlackboard 0) (Utilities|Name|MakeLiteralName "CanMove") false)
    (Class|PaperZDAnimInstance|JumptoNode (Class|PaperZDCharacter|GetAnimInstance) "JumpSpecialAttack" "None")))

(fn TurntoTarget
  (params (CustomTarget :type Boolean) (CustomTargetPosition :type Vector))
  (bind _asbp_pog_character_base (Utilities|Casting|CastToBP_Pog_Character_BASE (AI|Components|Blackboard|GetValueasObject (AI|GetBlackboard 0) (Utilities|Name|MakeLiteralName "Target"))))
  (if (< (select CustomTarget (.x (Variables|Default|GetSmartLinkDestination)) (.x (Transformation|GetActorLocation _asbp_pog_character_base))) (.x (Transformation|GetActorLocation)))
    (Transformation|SetActorRotation "0.000000,180.000000,0.000000")
    (else
      (Transformation|SetActorRotation "0, 0, 0"))))

(fn StartSpecialAttackCooldownTimer
  (Utilities|Time|SetTimerbyEvent (EventDispatchers|CreateEvent :!event EnableSpecialAttack) 8.0))

(fn EnableSpecialAttack
  (AI|Components|Blackboard|SetValueasBool (AI|GetBlackboard 0) (Utilities|Name|MakeLiteralName "IsSpecialAttackOnCD") false))

(fn PerformJumpOverGap
  (params (DestinationPos :type Vector) (ArcParam :type Float%20%28double-precision%29))
  ;[0.15 0.15 0.15 0.5] Отключение передвижения
  (AI|Components|Blackboard|SetValueasBool (AI|GetBlackboard 0) (Utilities|Name|MakeLiteralName "CanMove") false)
  (Variables|Default|SetCanMove false)
  ;[0.15 0.15 0.15 0.5] Остановка персонажа
  (AI|Navigation|StopMovement (AI|GetAIController self))
  ;[0.15 0.15 0.15 0.5] Рассчёт дуги для прыжка ИИ
  (bind _outlaunchvelocity (Game|SuggestProjectileVelocityCustomArc (Transformation|GetActorLocation) DestinationPos (Components|Movement|GetGravityZ (Variables|Character|GetCharacterMovement)) ArcParam))
  ;[0.15 0.15 0.15 0.5] Прыжок
  (Character|LaunchCharacter _outlaunchvelocity true true))

(fn EnemyStuckCheck
  (params (DeltaSeconds :type Float%20%28double-precision%29))
  (if (Math|Boolean|ANDBoolean (<= (Math|Vector|VectorLength (Variables|/Script/Engine.MovementComponent|GetVelocity (Variables|Character|GetCharacterMovement))) 0.0) (Variables|Default|GetCanMove) (or (not (Variables|Default|GetIsAttacking)) (not (Variables|Default|GetIsStunned))))
    (bind _output_get (Variables|Default|SetTimeWithoutMovement (+ (Variables|Default|GetTimeWithoutMovement) DeltaSeconds)))
    (if (>= _output_get (Variables|Default|GetTimeWithoutMovementToLaunch))
      (Utilities|FlowControl|DoOnce false :!label _label
        (:Completed
          (Character|LaunchCharacter (Math|Vector|MakeVector (* (Math|Float|SelectFloat 1.0 -1.0 (> (.x (Math|Vector|GetForwardVector (Math|Rotator|FindLookatRotation (Transformation|GetActorLocation self) (Transformation|GetActorLocation (Game|GetPlayerCharacter 0))))) 0.0)) 5e+02) 0.0 3e+02) true true)
          (Variables|Default|SetTimeWithoutMovement 0.0)
          (goto _label Reset))))
    (else
      (Variables|Default|SetTimeWithoutMovement 0.0))))