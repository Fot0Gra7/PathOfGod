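; BP_Ocelot is an enemy character that tells its AI when the player is within melee range.
; Overlaps on MeleeAttackTrigger with BP_Player_Keco set the IsInMeleeRange blackboard bool, true on entry and false on exit.
; The exit handler first checks that the blackboard is valid, avoiding errors when the AI dies.
; BeginPlay, ActorBeginOverlap and Tick are disabled stubs, and the construction script only calls its parent.
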(event OnComponentBeginOverlap(MeleeAttackTrigger)
  (params (OverlappedComponent :type Primitive%20Component%20Object%20Reference) (OtherActor :type Actor%20Object%20Reference) (OtherComp :type Primitive%20Component%20Object%20Reference) (OtherBodyIndex :type Integer) (bFromSweep :type Boolean) (SweepResult :type Hit%20Result%20Structure%20%28by%20ref%29))
  (Utilities|Casting|CastToBP_Player_Keco OtherActor)
  (AI|Components|Blackboard|SetValueasBool (AI|GetBlackboard 0) (Utilities|Name|MakeLiteralName "IsInMeleeRange") true))

(event OnComponentEndOverlap(MeleeAttackTrigger)
  (params (OverlappedComponent :type Primitive%20Component%20Object%20Reference) (OtherActor :type Actor%20Object%20Reference) (OtherComp :type Primitive%20Component%20Object%20Reference) (OtherBodyIndex :type Integer))
  ;[0 0.03125 0.01827 1 14] Чтобы не было ошибок при смерти ИИ
  (Utilities|IsValid (AI|GetBlackboard 0)
    (:Is%20Valid
      (Utilities|Casting|CastToBP_Player_Keco OtherActor)
      (AI|Components|Blackboard|SetValueasBool (AI|GetBlackboard 0) (Utilities|Name|MakeLiteralName "IsInMeleeRange") false))))

(event EventBeginPlay
  (|CallParentFunction) ; This node is disabled and will not be called.\nDrag off pins to build functionality.
)

(event Collision|EventActorBeginOverlap
  (params (OtherActor :type Actor%20Object%20Reference))
  (|CallParentFunction OtherActor) ; This node is disabled and will not be called.\nDrag off pins to build functionality.
)

(event EventTick
  (params (DeltaSeconds :type Float%20%28single-precision%29))
  (|CallParentFunction DeltaSeconds) ; This node is disabled and will not be called.\nDrag off pins to build functionality.
)

(fn ConstructionScript
  (|CallParentFunction))