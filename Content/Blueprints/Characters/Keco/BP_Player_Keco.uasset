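; Player character Blueprint for Keco in a side-scrolling sprite game, handling movement, combat and the health HUD.
; Enhanced Input drives movement, jumping, ground and air melee with hitboxes, and a hold-to-charge spear throw with flash tiers and cooldown.
; Tick line-traces for wall slides, enabling wall jumps that temporarily zero falling lateral friction.
; Damage interrupts charging and attacks, triggering knockback, stun and flickering invincibility that ignores Pawn collisions.
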(event OnComponentBeginOverlap(CapsuleComponent)
  (params (OverlappedComponent :type Primitive%20Component%20Object%20Reference) (OtherActor :type Actor%20Object%20Reference) (OtherComp :type Primitive%20Component%20Object%20Reference) (OtherBodyIndex :type Integer) (bFromSweep :type Boolean) (SweepResult :type Hit%20Result%20Structure%20%28by%20ref%29))
  (bind _asbp_pog_enemy_base (Utilities|Casting|CastToBP_Pog_Enemy_BASE OtherActor))
  ;[0 0.05208 0.003203 1 14] Проверка на капсулу, чтобы получать урон только от врагов
  (if (== (Variables|/Script/Engine.Character|GetCapsuleComponent _asbp_pog_enemy_base) OtherComp)
    (Game|Damage|ApplyDamage self (Variables|Vitality|GetOverlapDamage) 0 _asbp_pog_enemy_base)))

(event OnComponentBeginOverlap(Hitbox)
  (params (OverlappedComponent :type Primitive%20Component%20Object%20Reference) (OtherActor :type Actor%20Object%20Reference) (OtherComp :type Primitive%20Component%20Object%20Reference) (OtherBodyIndex :type Integer) (bFromSweep :type Boolean) (SweepResult :type Hit%20Result%20Structure%20%28by%20ref%29))
  (bind _asbp_pog_character_base (Utilities|Casting|CastToBP_Pog_Character_BASE OtherActor))
  (Default|KnockbackEnemy _asbp_pog_character_base _asbp_pog_character_base self))

(event OnComponentBeginOverlap(JumpHitbox)
  (params (OverlappedComponent :type Primitive%20Component%20Object%20Reference) (OtherActor :type Actor%20Object%20Reference) (OtherComp :type Primitive%20Component%20Object%20Reference) (OtherBodyIndex :type Integer) (bFromSweep :type Boolean) (SweepResult :type Hit%20Result%20Structure%20%28by%20ref%29))
  ;[0.004016 0.02083 0] Простая копирка нанесения урона из общего класса
  (bind _asbp_pog_character_base (Utilities|Casting|CastToBP_Pog_Character_BASE OtherActor))
  (if (Utilities|Enum|NotEqual(Enum) (Variables|/Game/Blueprints/Characters/BP_Pog_Character_BASE.BP_Pog_Character_BASE_C|GetFaction _asbp_pog_character_base) (Variables|Default|GetFaction))
    (Game|Damage|ApplyDamage _asbp_pog_character_base 1.0 0 self)
    (CallFunction|HitStopSequence 0.2)
    (CallFunction|HitStopSequence 0.2)))

(event Custom|GameOverScreen
  ;[1 0.03653 0 1 14] Здесь потом надо логику на поражение
)

(event Custom|TriggerInvincibility
  ;[0.000171 0.005208 0] Кадры неуязвимости
  ;;[0 0.006663 0.03646 1 12] Игнорирование коллизий других живых объектов игроком
  (Collision|SetCollisionResponsetoChannel (Variables|Default|GetCapsuleComponent) "ECC_Pawn" "ECR_Ignore")
  ;;[0 0.01562 0.01136 1 17] Включаем/выключаем видимость спрайта в функции по таймеру
  (bind _returnvalue (Utilities|Time|SetTimerbyEvent (EventDispatchers|CreateEvent :!event ToggleSpriteFlicker) (Variables|Vitality|GetSpriteFlickerInterval) true))
  (Variables|Vitality|SetFlickerHandle _returnvalue)
  ;;[0 0.01562 0.001406 1 17] Сколько ждать до выключения
  (Utilities|FlowControl|RetriggerableDelay (Variables|Vitality|GetInvincibilityDuration))
  ;;[0 0.0142 0.03125] Выключаем мерцание
  (Utilities|Time|ClearandInvalidateTimerbyHandle (Variables|Vitality|GetFlickerHandle))
  ;;[0 0.01042 0.000581 1 12] Возвращаем игроку возможность столкновений с врагами
  (Collision|SetCollisionResponsetoChannel (Variables|Default|GetCapsuleComponent) "ECC_Pawn" "ECR_Overlap")
  ;;[0 0.007658 0.02083 1 14] Включаем видимость в конце, чтобы персонаж не остался невидимым
  (Rendering|SetVisibility (Variables|Default|GetSprite) true false))

(event Custom|RestartChargeLoop
  ;[0 0.01562 0.001918 1 17] Do Once - чтобы анимация начала проигрываться, а не застревала на одном кадре, пока игрок удерживает клавишу
  (Utilities|FlowControl|DoOnce false) ; enters at Reset
)

(event Custom|ResetSpear
  ;[0 0.02083 0.002892] Таймер-КД на бросок
  (Variables|SpearThrow|SetIsSpearOnCD false)
  (Utilities|Time|ClearandInvalidateTimerbyHandle (Variables|SpearThrow|GetSpearCDTimer)))

(event Input|EnhancedActionEvents|EnhancedInputActionIA_Move
  (params (ActionValue :type Vector%202D%20Structure) (ElapsedSeconds :type Float%20%28double-precision%29) (TriggeredSeconds :type Float%20%28double-precision%29) (InputAction :type Input%20Action%20Object%20Reference :default "/Game/Input/Actions/IA_Move.IA_Move"))
  ;[0 0.01208 0.01562 1 16] Стандартное передвижение, можем поворачиваться пока заряжаем бросок копья.
  ; После добавления ближней атаки, возможность поворота во время неё убрать
  (if (and (not (Variables|Default|GetIsStunned)) (not (Variables|Default|GetIsAttacking)))
    ;;[0 0.03646 0.002477 1 12] Изменение направления взгляда персонажа
    (CallFunction|UpdateRotation (.x ActionValue))
    (if (Variables|Default|GetCanMove)
      (Pawn|Input|AddMovementInput "1.000000,0.000000,0.000000" (.x ActionValue) false)
      (else
        ;[0 0.007812 0.03125] Возможность двигаться и менять направление взгляда, пока игрок находится в прыжке (падении)
        (if (AI|Components|NavMovement|IsFalling (Variables|Character|GetCharacterMovement)) :!label _label
          (Pawn|Input|AddMovementInput "1.000000,0.000000,0.000000" (.x ActionValue) false)
          (if (Variables|SpearThrow|GetIsCharging)
            ;;[0 0.03646 0.002477 1 12] Изменение направления взгляда персонажа
            (CallFunction|UpdateRotation (.x ActionValue))))))
    (else
      (goto _label))))

(event Input|EnhancedActionEvents|EnhancedInputActionIA_Jump
  (params (ActionValue :type Boolean) (ElapsedSeconds :type Float%20%28double-precision%29) (TriggeredSeconds :type Float%20%28double-precision%29) (InputAction :type Input%20Action%20Object%20Reference :default "/Game/Input/Actions/IA_Jump.IA_Jump"))
  (:Started
    (if (Math|Boolean|ANDBoolean (not (Variables|Default|GetIsStunned)) (not (Variables|SpearThrow|GetIsCharging)) (not (Variables|Default|GetIsAttacking)))
      (if (Variables|WallJumping|GetIsWallSliding)
        (|WallJump)
        (else
          ;[0.01217 0.01562 0] Обычный прыжок
          (if (AI|Components|NavMovement|IsMovingonGround (Variables|Character|GetCharacterMovement))
            (Character|Jump))))))
  (:Canceled
    (Character|StopJumping :!label _label))
  (:Completed
    (goto _label)))

(event Input|EnhancedActionEvents|EnhancedInputActionIA_Shoot
  (params (ActionValue :type Boolean) (ElapsedSeconds :type Float%20%28double-precision%29) (TriggeredSeconds :type Float%20%28double-precision%29) (InputAction :type Input%20Action%20Object%20Reference :default "/Game/Input/Actions/IA_Shoot.IA_Shoot"))
  (:Started
    (if (not (Variables|Default|GetIsStunned))
      (Variables|SpearThrow|SetWasHitDuringCharge false)
      (Variables|Default|SetCanThrowSpear true)))
  (:Ongoing
    (if (Math|Boolean|ANDBoolean (not (Variables|Default|GetIsStunned)) (not (Variables|SpearThrow|GetWasHitDuringCharge)) (not (Variables|SpearThrow|GetIsSpearOnCD)) (Variables|Default|GetCanThrowSpear))
      (CallFunction|HandleChargeFlash ElapsedSeconds)
      (Variables|Default|SetCanMove false)
      (Variables|SpearThrow|SetIsCharging true)
      ;[0 0.01562 0.001918 1 17] Do Once - чтобы анимация начала проигрываться, а не застревала на одном кадре, пока игрок удерживает клавишу
      (Utilities|FlowControl|DoOnce false
        (:Completed
          (Class|PaperZDAnimInstance|JumptoNode (Variables|/Script/PaperZD.PaperZDAnimationComponent|GetAnimInstance (Variables|Default|GetAnimationComponent)) "JumpSpearThrowCharge" "None")))
      (else
        ;[0 0.05208 0.03149 1 12] Чтобы игрок не мог заряжать бросок копья, пока оно находится в КД.
        (Variables|Default|SetCanThrowSpear false)
        (Development|PrintString "копьё прбн" true true "(R=0.000000,G=0.660000,B=1.000000,A=1.000000)" 0.2))))
  (:Completed
    (if (Math|Boolean|ANDBoolean (not (Variables|Default|GetIsStunned)) (Variables|SpearThrow|GetIsCharging) (not (Variables|SpearThrow|GetWasHitDuringCharge)))
      (CallFunction|TryChargeThrow ElapsedSeconds)
      (Class|PaperZDAnimInstance|JumptoNode (Variables|/Script/PaperZD.PaperZDAnimationComponent|GetAnimInstance (Variables|Default|GetAnimationComponent)) "JumpSpearThrowEnd" "None")
      ;[0 0.02083 0.002892] Таймер-КД на бросок
      (if (Variables|SpearThrow|GetIsSpearOnCD)
        (bind _returnvalue (Utilities|Time|SetTimerbyEvent (delegate Custom|ResetSpear) (Variables|SpearThrow|GetSpearThrowCD)))
        (Variables|SpearThrow|SetSpearCDTimer _returnvalue)))))

(event Input|EnhancedActionEvents|EnhancedInputActionIA_Attack
  (params (ActionValue :type Boolean) (ElapsedSeconds :type Float%20%28double-precision%29) (TriggeredSeconds :type Float%20%28double-precision%29) (InputAction :type Input%20Action%20Object%20Reference :default "/Game/Input/Actions/IA_Attack.IA_Attack"))
  (:Started
    (if (Math|Boolean|ANDBoolean (not (Variables|Default|GetIsAttacking)) (not (Variables|Default|GetIsStunned)) (not (Variables|SpearThrow|GetIsCharging)))
      ;[0 0.009695 0.01042] На земле ли игрок
      (if (not (AI|Components|NavMovement|IsFalling (Variables|Character|GetCharacterMovement)))
        ;[0.001126 0.01042 0] Обычная атака (на земле)
        (|PlayAnimationOverridewithCallbacks (Class|PaperZDCharacter|GetAnimInstance) "/Game/Blueprints/Characters/Keco/AnimSequences/Attack.Attack" "DefaultSlot" 1.0 0.0
          (:then
            (Variables|Default|SetIsAttacking true)
            (Variables|Default|SetCanMove false))
          (:OnCompleted
            (Variables|Default|SetIsAttacking false :!label _label)
            (Variables|Default|SetCanMove true))
          (:OnCancelled
            (goto _label)))
        (else
          ;[0.000304 0.004025 0] Атака в воздухе
          (|PlayAnimationOverridewithCallbacks (Class|PaperZDCharacter|GetAnimInstance) "/Game/Blueprints/Characters/Keco/AnimSequences/JumpAttack.JumpAttack" "DefaultSlot" 1.0 0.0
            (:then
              (Variables|Default|SetIsAttacking true)
              (Variables|Default|SetCanMove false))
            (:OnCompleted
              (Variables|Default|SetIsAttacking false :!label _label_2)
              (Variables|Default|SetCanMove true))
            (:OnCancelled
              (goto _label_2))))))))

(event EventBeginPlay
  (|CallParentFunction)
  (Utilities|FlowControl|Sequence
    (:then_0
      ;[0 0.02981 0.03646] Получение ссылки на гейммод
      (bind _asgm_keco (Utilities|Casting|CastToGM_Keco (Game|GetGameMode)))
      (Variables|Default|SetGameModeMain _asgm_keco)
      ;[0.000475 0.02083 0] Подключения управления персонажу (IMC - Input Mapping Context)
      (bind _asplayer_controller (Utilities|Casting|CastToPlayerController (Pawn|GetController)))
      (Input|AddMappingContext (PlayerController|LocalPlayerSubsystems|GetEnhancedInputLocalPlayerSubsystem _asplayer_controller) "/Game/Input/IMC_Action.IMC_Action" 0 "(bIgnoreAllPressedKeysUntilRelease=True,bForceImmediately=False,bNotifyUserSettings=False)"))
    (:then_1
      ;[0.003245 0.02083 0 1 16] Запоминание стандартного значения управляемости в воздухе
      (Variables|Default|SetBaseLateralFriction (Variables|/Script/Engine.CharacterMovementComponent|GetFallingLateralFriction (Variables|Character|GetCharacterMovement)))
      ;[0 0.02604 0.000944] Обновляем виджет со здоровьем после появления персонажа
      (Default|UpdateHealth (Variables|/Game/Widgets/W_HUD.W_HUD_C|GetW_HealthComponent (Variables|/Game/Blueprints/GM_Keco.GM_Keco_C|GetHudWidget (Variables|Default|GetGameModeMain))) (Variables|/Game/Blueprints/Components/BPC_Vitality.BPC_Vitality_C|GetCurrentHealth (Variables|Default|GetBPC_Vitality))))
    (:then_2
      ;[1 0.03653 0 1 14] Здесь потом надо логику на поражение
      (EventDispatchers|BindEventtoDefeated (delegate Custom|GameOverScreen)))))

(event Collision|EventActorBeginOverlap
  (params (OtherActor :type Actor%20Object%20Reference))
  (|CallParentFunction OtherActor) ; This node is disabled and will not be called.\nDrag off pins to build functionality.
)

(event EventTick
  (params (DeltaSeconds :type Float%20%28single-precision%29))
  (|CallParentFunction DeltaSeconds)
  (CallFunction|TryWallSlide))

(event Game|Damage|EventAnyDamage
  (params (Damage :type Float%20%28single-precision%29) (DamageType :type Damage%20Type%20Object%20Reference) (InstigatedBy :type Controller%20Object%20Reference) (DamageCauser :type Actor%20Object%20Reference))
  (|CallParentFunction Damage DamageType InstigatedBy DamageCauser)
  ;[0 0.02331 0.03646] Выключение анимации атаки
  (Class|PaperZDAnimInstance|StopAllAnimationOverrides (Class|PaperZDCharacter|GetAnimInstance))
  (Default|UpdateHealth (Variables|/Game/Widgets/W_HUD.W_HUD_C|GetW_HealthComponent (Variables|/Game/Blueprints/GM_Keco.GM_Keco_C|GetHudWidget (Variables|Default|GetGameModeMain))) (Variables|/Game/Blueprints/Components/BPC_Vitality.BPC_Vitality_C|GetCurrentHealth (Variables|Default|GetBPC_Vitality)))
  (Variables|SpearThrow|SetWasHitDuringCharge true)
  (if (not (Variables|/Game/Blueprints/Components/BPC_Vitality.BPC_Vitality_C|GetIsDefeated (Variables|Default|GetBPC_Vitality)))
    (CallFunction|TriggerInvincibility)
    (Variables|SpearThrow|SetIsCharging false)
    (Variables|Default|SetCanMove true)
    (CallFunction|RestartChargeLoop)
    (|Knockback DamageCauser)))

(event EventOnLanded
  (params (Hit :type Hit%20Result%20Structure%20%28by%20ref%29))
  (if (Variables|Default|GetIsAttacking)
    ;[0 0.02331 0.03646] Выключение анимации атаки
    (Class|PaperZDAnimInstance|StopAllAnimationOverrides (Class|PaperZDCharacter|GetAnimInstance))))

(fn ConstructionScript
  (|CallParentFunction))

(fn UpdateRotation
  (params (Direction :type Float%20%28double-precision%29))
  (if (!= Direction 0.0)
    (Pawn|SetControlRotation (Pawn|GetController) (select (>= Direction 0.0) (Math|Rotator|MakeRotator 0.0 0.0 0.0) (Math|Rotator|MakeRotator 0.0 0.0 1.8e+02)))))

(fn TryWallSlide
  (bind _returnvalue (Transformation|GetActorLocation))
  ;[0 0.03137 0 1 15] Падаем ли вниз и удерживаем ли клавишу в сторону стены
  (if (Math|Boolean|ANDBoolean (|IsDescending) (|IsHoldingTowardsWall) (not (Variables|SpearThrow|GetIsCharging)) (not (Variables|Default|GetIsAttacking)))
    ;[0.000477 0.01562 0] Сталкивается ли персонаж со статичным объектами
    (bind _returnvalue_2 (Collision|LineTraceForObjects _returnvalue (+ _returnvalue (* (Transformation|GetActorForwardVector) (Variables|WallJumping|GetWallTraceLenght))) (Utilities|Array|MakeArray "ObjectTypeQuery1") false 0 "ForOneFrame"))
    (if _returnvalue_2
      (Variables|WallJumping|SetIsWallSliding true)
      ;[0.001055 0.01042 0 1 16] Изменение вертикальной скорости персонажа, пока он находится на стене
      (Variables|/Script/Engine.MovementComponent|SetVelocity (Variables|Character|GetCharacterMovement) (Math|Vector|MakeVector (.x (Variables|/Script/Engine.MovementComponent|GetVelocity (Variables|Character|GetCharacterMovement))) (.y (Variables|/Script/Engine.MovementComponent|GetVelocity (Variables|Character|GetCharacterMovement))) (Math|Float|Max(Float) (.z (Variables|/Script/Engine.MovementComponent|GetVelocity (Variables|Character|GetCharacterMovement))) (Variables|WallJumping|GetWallSlideSpeed))))
      (else
        (Variables|WallJumping|SetIsWallSliding false)))
    (else
      (Variables|WallJumping|SetIsWallSliding false))))

(fn ToggleSpriteFlicker
  (Rendering|SetVisibility (Variables|Default|GetSprite) (not (Variables|/Script/Engine.SceneComponent|GetbVisible (Variables|Default|GetSprite))) true))

(fn ThrowSpear
  (params (SpearType :type BP%20Player%20Spear%20BASE%20Class%20Reference))
  (bind _self self)
  (bind _spearthrowpos (Variables|Default|GetSpearThrowPos))
  (bind _returnvalue (Transformation|GetWorldTransform _spearthrowpos))
  (Game|SpawnActorfromClass SpearType (Math|Transform|MakeTransform (.location _returnvalue) (.rotation _returnvalue) "1.000000,1.000000,1.000000") "AlwaysSpawn" "MultiplyWithRoot" _self _self))

(fn TryChargeThrow
  (params (ElapsedTime :type Float%20%28double-precision%29))
  (if (and (not (Variables|SpearThrow|GetWasHitDuringCharge)) (>= ElapsedTime (Variables|SpearThrow|GetMinChargeTimeToThrowSpear)))
    (Variables|SpearThrow|SetIsSpearOnCD true)
    ;[7.9e-05 0.01562 0] Бросок медленного копья
    (if (>= ElapsedTime (Variables|SpearThrow|GetAverageThrowChargeTime))
      ;[0 0.01323 0.03646] Бросок среднего копья
      (if (>= ElapsedTime (Variables|SpearThrow|GetFastThrowChargeTime))
        ;[0.000281 0.02083 0] Бросок быстрого или полностью заряженного копья
        (if (>= ElapsedTime (Variables|SpearThrow|GetFullThrowChargeTime))
          (CallFunction|ThrowSpear "/Game/Blueprints/Projectiles/BP_PlayerSpear_FullCharge.BP_PlayerSpear_FullCharge_C")
          (else
            (CallFunction|ThrowSpear "/Game/Blueprints/Projectiles/BP_PlayerSpear_Fast.BP_PlayerSpear_Fast_C")))
        (else
          (CallFunction|ThrowSpear "/Game/Blueprints/Projectiles/BP_PlayerSpear_Average.BP_PlayerSpear_Average_C")))
      (else
        (CallFunction|ThrowSpear "/Game/Blueprints/Projectiles/BP_PlayerSpear_Slow.BP_PlayerSpear_Slow_C")))))

(fn HandleChargeFlash
  (params (ElapsedTime :type Float%20%28double-precision%29))
  (if (and (>= ElapsedTime (Variables|SpearThrow|GetAverageThrowChargeTime)) (not (Variables|SpearThrow|GetWasHitDuringCharge)))
    ;[0 0.01042 0.000331] Интервал мерцания
    (Variables|SpearThrow|SetChargeFlashTimer (+ (Variables|SpearThrow|GetChargeFlashTimer) (Utilities|Time|GetWorldDeltaSeconds)))
    (if (>= (Variables|SpearThrow|GetChargeFlashTimer) (Variables|SpearThrow|GetChargeFlashInterval))
      ;[0 0.002125 0.03071 1 16] Обнуление интервала
      (Variables|SpearThrow|SetChargeFlashTimer 0.0)
      (CallFunction|TriggerFlash 5.0 (select (>= ElapsedTime (Variables|SpearThrow|GetFullThrowChargeTime)) "(R=0.047747,G=0.458333,B=0.000000,A=1.000000)" (select (>= ElapsedTime (Variables|SpearThrow|GetFastThrowChargeTime)) "(R=0.005449,G=0.000000,B=1.000000,A=1.000000)" "(R=1.000000,G=1.000000,B=1.000000,A=1.000000)"))))
    (else
      ;[0 0.002125 0.03071 1 16] Обнуление интервала
      (Variables|SpearThrow|SetChargeFlashTimer 0.0))))

(fn SetJumpAttackHitboxCollision
  (params (SetActive :type Boolean))
  (if SetActive
    (Collision|SetCollisionEnabled (Variables|Default|GetJumpHitbox) "QueryOnly")
    (else
      (Collision|SetCollisionEnabled (Variables|Default|GetJumpHitbox) "NoCollision"))))