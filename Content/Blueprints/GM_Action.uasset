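; Game mode for the action game that sets up the HUD and handles checkpoint-based player respawning.
; BeginPlay caches the level's PlayerStart and adds the W_HUD widget to the viewport.
; RespawnPlayer spawns a new default pawn at the active checkpoint's Scene component, falling back to PlayerStart if none is valid.
; Player controller 0 then possesses the pawn, and a respawn sound plays.
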(event EventBeginPlay
  (bind _returnvalue (Actor|GetActorOfClass "/Script/Engine.PlayerStart"))
  (Variables|Default|SetPlayerStart _returnvalue)
  (bind _returnvalue_2 (UserInterface|CreateWidget "/Game/Widgets/W_HUD.W_HUD_C" (Game|GetPlayerController 0)))
  (bind _output_get (Variables|Default|SetHudWidget _returnvalue_2))
  (UserInterface|Viewport|AddtoViewport _returnvalue_2 0))

(event EventTick
  (params (DeltaSeconds :type Float%20%28single-precision%29)))

(fn ConstructionScript)

(fn RespawnPlayer
  (bind _playerstart (Variables|Default|GetPlayerStart))
  (bind _activecheckpoint (Variables|Default|GetActiveCheckpoint))
  (bind _returnvalue (Transformation|GetActorTransform _playerstart))
  (bind _scene (Variables|/Game/Blueprints/Props/ActionPlatformerProps/BP_Checkpoint.BP_Checkpoint_C|GetScene _activecheckpoint))
  (bind _returnvalue_2 (Transformation|GetWorldTransform _scene))
  (Utilities|IsValid (Variables|Default|GetActiveCheckpoint)
    (:Is%20Valid
      (bind _returnvalue_3 (Game|SpawnActorfromClass (Variables|Default|GetDefaultPawnClass) (Math|Transform|MakeTransform (.location _returnvalue_2) (.rotation _returnvalue_2) "1.000000,1.000000,1.000000") "AlwaysSpawn" "MultiplyWithRoot" 0 0))
      (Pawn|Possess (Game|GetPlayerController 0) _returnvalue_3)
      (Audio|PlaySound2D "/Game/Audio/SFX/Respawn_Player_Cue.Respawn_Player_Cue" 1.0 1.0 0.0 0 0))
    (:Is%20Not%20Valid
      (bind _returnvalue_4 (Game|SpawnActorfromClass (Variables|Default|GetDefaultPawnClass) (Math|Transform|MakeTransform (.location _returnvalue) (.rotation _returnvalue) "1.000000,1.000000,1.000000") "AlwaysSpawn" "MultiplyWithRoot" 0 0))
      (Pawn|Possess (Game|GetPlayerController 0) _returnvalue_4)
      (Audio|PlaySound2D "/Game/Audio/SFX/Respawn_Player_Cue.Respawn_Player_Cue" 1.0 1.0 0.0 0 0))))