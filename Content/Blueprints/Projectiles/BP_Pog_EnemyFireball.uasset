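; Enemy fireball projectile that damages opposing-faction characters and bursts on impact.
; It spawns a Niagara trail at BeginPlay and moves it to the projectile every tick.
; Overlap with a tagged character hitbox applies damage through a DoOnce, spawns the impact effect and destroys the actor.
; A blocking hit on the trigger spawns the same effect, plays a hit sound and destroys it without damage.
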(event OnComponentBeginOverlap(DamageTrigger)
  (params (OverlappedComponent :type Primitive%20Component%20Object%20Reference) (OtherActor :type Actor%20Object%20Reference) (OtherComp :type Primitive%20Component%20Object%20Reference) (OtherBodyIndex :type Integer) (bFromSweep :type Boolean) (SweepResult :type Hit%20Result%20Structure%20%28by%20ref%29))
  (Utilities|FlowControl|Sequence
    (:then_0
      (bind _asbp_pog_character_base (Utilities|Casting|CastToBP_Pog_Character_BASE OtherActor))
      (if (and (Utilities|Enum|NotEqual(Enum) (Variables|/Game/Blueprints/Characters/BP_Pog_Character_BASE.BP_Pog_Character_BASE_C|GetFaction _asbp_pog_character_base) (Variables|Default|GetE_Faction)) (Components|ComponentHasTag OtherComp "CharacterHitbox"))
        (Utilities|FlowControl|DoOnce false
          (:Completed
            (Game|Damage|ApplyDamage _asbp_pog_character_base 1.0 0 self)
            (CallFunction|ResetDamage)
            (Niagara|SpawnSystematLocation "/Game/VFX/NS_FireBall_Impact.NS_FireBall_Impact" (Transformation|GetActorLocation))
            (Actor|DestroyActor)))))))

(event OnComponentHit(DamageTrigger)
  (params (HitComponent :type Primitive%20Component%20Object%20Reference) (OtherActor :type Actor%20Object%20Reference) (OtherComp :type Primitive%20Component%20Object%20Reference) (NormalImpulse :type Vector :default "0, 0, 0") (Hit :type Hit%20Result%20Structure%20%28by%20ref%29))
  (Niagara|SpawnSystematLocation "/Game/VFX/NS_FireBall_Impact.NS_FireBall_Impact" (Transformation|GetActorLocation))
  (Audio|PlaySound2D "/Game/Audio/SFX_Igor/Fireball/SC_Hit_Fireball.SC_Hit_Fireball" 1.0 1.0 0.0 0 0)
  (Actor|DestroyActor))

(event Custom|ResetDamage
  (Utilities|FlowControl|DoOnce false) ; enters at Reset
)

(event EventBeginPlay
  (|CallParentFunction)
  (bind _returnvalue (Niagara|SpawnSystematLocation "/Game/VFX/NS_FireBall_Trail.NS_FireBall_Trail" (Transformation|GetActorLocation)))
  (Variables|Default|SetTrail _returnvalue))

(event EventTick
  (params (DeltaSeconds :type Float%20%28single-precision%29))
  (|CallParentFunction DeltaSeconds)
  (Transformation|SetWorldLocation (Variables|Default|GetTrail) (Transformation|GetActorLocation) false false))

(fn ConstructionScript
  (|CallParentFunction))