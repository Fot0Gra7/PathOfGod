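; Base projectile Blueprint that can be reflected and destroys itself on impact.
; On BeginPlay it records an offset spawn position, which ProjectileReflection uses as a return target for the Enemy faction, while Player follows the supplied forward vector.
; Reflection also sets a new max speed and velocity and removes gravity.
; A DamageTrigger hit spawns VFX and plays a sound before destruction, without applying damage here.
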(event OnComponentHit(DamageTrigger)
  (params (HitComponent :type Primitive%20Component%20Object%20Reference) (OtherActor :type Actor%20Object%20Reference) (OtherComp :type Primitive%20Component%20Object%20Reference) (NormalImpulse :type Vector :default "0, 0, 0") (Hit :type Hit%20Result%20Structure%20%28by%20ref%29))
  (CallFunction|PlayHitEffects)
  (Actor|DestroyActor))

(event EventBeginPlay
  (Variables|Default|SetProjectileSpawnPosition (+ (Transformation|GetActorLocation) (Variables|Default|GetProjectileStartPosOffset))))

(event Collision|EventActorBeginOverlap
  (params (OtherActor :type Actor%20Object%20Reference)))

(event EventTick
  (params (DeltaSeconds :type Float%20%28single-precision%29)))

(fn ConstructionScript)

(fn ProjectileReflection
  (params (ForwardVector :type Vector) (ReflectorPosition :type Vector))
  (bind _projectilemovement (Variables|Default|GetProjectileMovement))
  (Variables|/Script/Engine.ProjectileMovementComponent|SetMaxSpeed _projectilemovement (Variables|Default|GetMaxReflectionSpeed))
  (Variables|/Script/Engine.MovementComponent|SetVelocity _projectilemovement (* (Utilities|Select :Index (Variables|Default|GetE_Faction) :NewEnumerator0 ForwardVector :NewEnumerator1 (Math|Vector|Normalize (- (Variables|Default|GetProjectileSpawnPosition) ReflectorPosition))) (Variables|Default|GetReflectionVelocity)))
  (Variables|/Script/Engine.ProjectileMovementComponent|SetProjectileGravityScale _projectilemovement 0.0))

(fn PlayHitEffects
  (Game|SpawnActorfromClass "/Game/Blueprints/VFX/BP_VFX_ShotHit.BP_VFX_ShotHit_C" (Math|Transform|MakeTransform (Transformation|GetActorLocation) (Transformation|GetActorRotation) "1.000000,1.000000,1.000000") "AlwaysSpawn" "MultiplyWithRoot" 0 0)
  (Audio|PlaySoundatLocation "/Game/Audio/SFX/Destroyed_Projectile_Cue.Destroyed_Projectile_Cue" (Transformation|GetActorLocation) "0, 0, 0" 1.0 1.0 0.0 0 0 0 0))