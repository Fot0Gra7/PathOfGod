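; Base spear projectile that damages characters of another faction on contact.
; When its Box overlaps a BP_Pog_Character_BASE whose faction differs from its own, it applies projectile damage, plays hit effects and destroys itself.
; On a Box hit, it compares the surface normal with the spear's up vector by dot product to tell floor from wall, currently only printing the result.
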(event OnComponentHit(Box)
  (params (HitComponent :type Primitive%20Component%20Object%20Reference) (OtherActor :type Actor%20Object%20Reference) (OtherComp :type Primitive%20Component%20Object%20Reference) (NormalImpulse :type Vector :default "0, 0, 0") (Hit :type Hit%20Result%20Structure%20%28by%20ref%29))
  (if (> (Math|Vector|DotProduct (.Normal (Collision|BreakHitResult Hit)) (Math|Vector|GetUpVector (Transformation|GetActorRotation))) 0.5)
    (Development|PrintString "Пол")
    (else
      (Development|PrintString "Стена" true true "(R=1.000000,G=0.078249,B=0.000000,A=1.000000)"))))

(event OnComponentBeginOverlap(Box)
  (params (OverlappedComponent :type Primitive%20Component%20Object%20Reference) (OtherActor :type Actor%20Object%20Reference) (OtherComp :type Primitive%20Component%20Object%20Reference) (OtherBodyIndex :type Integer) (bFromSweep :type Boolean) (SweepResult :type Hit%20Result%20Structure%20%28by%20ref%29))
  (Utilities|FlowControl|Sequence
    (:then_0
      (bind _asbp_pog_character_base (Utilities|Casting|CastToBP_Pog_Character_BASE OtherActor))
      (if (Utilities|Enum|NotEqual(Enum) (Variables|/Game/Blueprints/Characters/BP_Pog_Character_BASE.BP_Pog_Character_BASE_C|GetFaction _asbp_pog_character_base) (Variables|Default|GetE_Faction))
        (Game|Damage|ApplyDamage OtherActor (Variables|Default|GetProjectileDamage) 0 self)
        (CallFunction|PlayHitEffects)
        (Actor|DestroyActor)))))

(event EventBeginPlay)

(event Collision|EventActorBeginOverlap
  (params (OtherActor :type Actor%20Object%20Reference)))

(event EventTick
  (params (DeltaSeconds :type Float%20%28single-precision%29)))

(fn ConstructionScript)