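; Camera bounds actor that keeps a camera target point following the player character while confined to a box volume.
; On BeginPlay it caches player character 0 as the target actor.
; Each Tick, ClampCameraPosition clamps the target's location per axis to the world bounds of CameraTargetMovementBox, and CameraTarget is moved there.
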(event EventBeginPlay
  (Variables|Default|SetTargetActor (Game|GetPlayerCharacter 0)))

(event Collision|EventActorBeginOverlap
  (params (OtherActor :type Actor%20Object%20Reference)))

(event EventTick
  (params (DeltaSeconds :type Float%20%28single-precision%29))
  (bind _return_vector (CallFunction|ClampCameraPosition (Transformation|GetActorLocation (Variables|Default|GetTargetActor))))
  (Transformation|SetWorldLocation (Variables|Default|GetCameraTarget) _return_vector false false))

(fn ConstructionScript)

(fn ClampCameraPosition
  (params (DesiredCameraPos%20 :type Vector))
  (bind (_x _y _z) (Math|Vector|BreakVector DesiredCameraPos%20))
  (bind _cameratargetmovementbox (Variables|Default|GetCameraTargetMovementBox))
  (bind (_origin _boxextent) (Collision|GetComponentBounds _cameratargetmovementbox))
  (bind _returnvalue (- _origin _boxextent))
  (bind _returnvalue_2 (+ _origin _boxextent))
  (return (Math|Vector|MakeVector (Math|Float|Clamp(Float) _x (.x _returnvalue) (.x _returnvalue_2)) (Math|Float|Clamp(Float) _y (.y _returnvalue) (.y _returnvalue_2)) (Math|Float|Clamp(Float) _z (.z _returnvalue) (.z _returnvalue_2)))))