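; BP_EnemySpawner is a placed spawner that periodically spawns random enemies at its own transform.
; On BeginPlay it rolls one interval, SpawnInterval plus a small random offset, and keeps it for a looping timer.
; Each tick of that timer picks a random allowed type and looks up its class in SpawnClasses, spawning regardless of collision.
; The lookup check and the spawn each roll separately, so their types can differ.
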(event Custom|SpawnEnemy
  (bind _allowedenemyspawntypes (Variables|Default|GetAllowedEnemySpawnTypes))
  (bind _allowedenemyspawntypes_2 (Variables|Default|GetAllowedEnemySpawnTypes))
  (bind _spawnclasses (Variables|Default|GetSpawnClasses))
  (bind _returnvalue (Utilities|Array|Length _allowedenemyspawntypes))
  (bind _returnvalue_2 (- _returnvalue 1))
  (bind _returnvalue_3 (Math|Random|RandomIntegerinRange 0 _returnvalue_2))
  (bind _output (Utilities|Array|Get(acopy) _allowedenemyspawntypes_2 _returnvalue_3))
  (bind (_value _returnvalue_4) (Utilities|Map|Find _spawnclasses _output))
  (if (> (Utilities|Array|Length (Variables|Default|GetAllowedEnemySpawnTypes)) 0)
    (if _returnvalue_4
      (Game|SpawnActorfromClass _value (Transformation|GetActorTransform) "AlwaysSpawn" "MultiplyWithRoot" 0 0))))

(event EventBeginPlay
  (Utilities|Time|SetTimerbyEvent (delegate Custom|SpawnEnemy) (Math|Random|RandomFloatinRange (Variables|Default|GetSpawnInterval) (+ (Variables|Default|GetSpawnInterval) 3.0)) true))

(event Collision|EventActorBeginOverlap
  (params (OtherActor :type Actor%20Object%20Reference)))

(event EventTick
  (params (DeltaSeconds :type Float%20%28single-precision%29)))

(fn ConstructionScript)