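; Gate prop that opens on begin game or, when flagged as the exit, on quest completion.
; On BeginPlay, IsThisGateExit decides which of those two events OpenGate binds to.
; A timeline, rate-scaled by GateOpeningTime in seconds, lerps the door sprite from its local origin to the OpenLocation component's relative position.
; CloseGate plays the same timeline in reverse from the end.
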(event Custom|OpenGate
  (Components|Timeline|SetPlayRate (Variables|Default|GetOpenTheGate) (/ 1.0 (Variables|Default|GetGateOpeningTime)))
  (bind _gateopening (Timeline|OpenTheGate PlayFromStart)
    (:Update
      (Transformation|SetRelativeLocation (Variables|Default|GetDoor_Sprite) (Math|Vector|Lerp(Vector) "0, 0, 0" (Variables|/Script/Engine.SceneComponent|GetRelativeLocation (Variables|Default|GetOpenLocation)) _gateopening) false false))))

(event Custom|CloseGate
  (Components|Timeline|SetPlayRate (Variables|Default|GetOpenTheGate) (/ 1.0 (Variables|Default|GetGateOpeningTime)))
  (bind _gateopening (Timeline|OpenTheGate ReverseFromEnd)
    (:Update
      (Transformation|SetRelativeLocation (Variables|Default|GetDoor_Sprite) (Math|Vector|Lerp(Vector) "0, 0, 0" (Variables|/Script/Engine.SceneComponent|GetRelativeLocation (Variables|Default|GetOpenLocation)) _gateopening) false false))))

(event EventBeginPlay
  (Utilities|FlowControl|Sequence
    (:then_0
      (if (not (Variables|Default|GetIsThisGateExit))
        (EventDispatchers|BindEventtoBeginGame (delegate Custom|OpenGate))))
    (:then_1
      (if (Variables|Default|GetIsThisGateExit)
        (EventDispatchers|BindEventtoQuestCompleted (delegate Custom|OpenGate))))))

(event Collision|EventActorBeginOverlap
  (params (OtherActor :type Actor%20Object%20Reference)))

(event EventTick
  (params (DeltaSeconds :type Float%20%28single-precision%29)))

(fn ConstructionScript)