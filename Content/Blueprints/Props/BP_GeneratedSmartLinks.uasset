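; BP_GeneratedSmartLinks is a generated nav smart link that makes enemies jump when they reach it during pathfinding.
; On reach, it accepts only BP_Pog_Enemy_BASE agents and hands them itself and the link destination.
; It then halts their AI movement, clears CanMove on both pawn and blackboard, and jumps the anim instance to the jump-start node, leaving the traversal to the enemy.
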(event EventSmartLinkReached
  (params (Agent :type Actor%20Object%20Reference) (Destination :type Vector :default "0, 0, 0"))
  (bind _asbp_pog_enemy_base (Utilities|Casting|CastToBP_Pog_Enemy_BASE Agent))
  (Variables|/Game/Blueprints/Characters/Enemies/BP_Pog_Enemy_BASE.BP_Pog_Enemy_BASE_C|SetCurrentGeneratedLink _asbp_pog_enemy_base self)
  (Variables|/Game/Blueprints/Characters/Enemies/BP_Pog_Enemy_BASE.BP_Pog_Enemy_BASE_C|SetSmartLinkDestination _asbp_pog_enemy_base Destination)
  (Variables|/Game/Blueprints/Characters/BP_Pog_Character_BASE.BP_Pog_Character_BASE_C|SetCanMove _asbp_pog_enemy_base false)
  (AI|Components|Blackboard|SetValueasBool (AI|GetBlackboard _asbp_pog_enemy_base) (Utilities|Name|MakeLiteralName "CanMove") false)
  (AI|Navigation|StopMovement (AI|GetAIController _asbp_pog_enemy_base))
  (Variables|/Game/Blueprints/Characters/Enemies/BP_Pog_Enemy_BASE.BP_Pog_Enemy_BASE_C|SetIsInJumpAnim _asbp_pog_enemy_base true)
  (Class|PaperZDAnimInstance|JumptoNode (Class|PaperZDCharacter|GetAnimInstance _asbp_pog_enemy_base) "JumpStartJump" "None"))