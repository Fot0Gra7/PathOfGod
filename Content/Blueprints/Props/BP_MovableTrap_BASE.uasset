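; Base movable trap or turret that slides a Paper2D flipbook along a spline and keeps its shoot position aimed at the player.
; Each tick, the movement variation advances a normalized spline key as ping-pong or looping in either direction, or runs Clear Shot mode.
; Clear Shot line-traces from sampled spline points to pick one near the player with an unblocked view, then interpolates the trap's spline distance toward it.
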(event EventBeginPlay
  (|CallParentFunction)
  (Variables|Default|SetSplineLength (Spline|GetSplineLength (Variables|Default|GetSpline))))

(event Collision|EventActorBeginOverlap
  (params (OtherActor :type Actor%20Object%20Reference))
  (|CallParentFunction OtherActor) ; This node is disabled and will not be called.\nDrag off pins to build functionality.
)

(event EventTick
  (params (DeltaSeconds :type Float%20%28single-precision%29))
  (|CallParentFunction DeltaSeconds)
  (Utilities|FlowControl|Sequence
    (:then_0
      (switch Utilities|FlowControl|Switch|SwitchonE_Trap_Movement_Variation (Variables|Default|GetMovementVariation)
        (:NewEnumerator0
          ;[0 0.003766 0.01042] Ping Pong movement
          (if (Variables|Default|GetIsMovingForward)
            (if (>= (+ (Variables|Default|GetCurrentSplineKey) (* (Variables|Default|GetMovementSpeed) DeltaSeconds)) 1.0)
              (Variables|Default|SetCurrentSplineKey 1.0)
              (Variables|Default|SetIsMovingForward false)
              (else
                (Variables|Default|SetCurrentSplineKey (+ (Variables|Default|GetCurrentSplineKey) (* (Variables|Default|GetMovementSpeed) DeltaSeconds)))))
            (elif (<= (- (Variables|Default|GetCurrentSplineKey) (* (Variables|Default|GetMovementSpeed) DeltaSeconds)) 0.0)
              (Variables|Default|SetCurrentSplineKey 0.0)
              (Variables|Default|SetIsMovingForward true)
              (else
                (Variables|Default|SetCurrentSplineKey (- (Variables|Default|GetCurrentSplineKey) (* (Variables|Default|GetMovementSpeed) DeltaSeconds)))))))
        (:NewEnumerator1
          ;[0 0.01953 0.02083] Clockwise movement
          (if (> (+ (Variables|Default|GetCurrentSplineKey) (* (Variables|Default|GetMovementSpeed) DeltaSeconds)) 1.0)
            (Variables|Default|SetCurrentSplineKey (- (+ (Variables|Default|GetCurrentSplineKey) (* (Variables|Default|GetMovementSpeed) DeltaSeconds)) 1.0))
            (else
              (Variables|Default|SetCurrentSplineKey (+ (Variables|Default|GetCurrentSplineKey) (* (Variables|Default|GetMovementSpeed) DeltaSeconds))))))
        (:NewEnumerator2
          ;[0 0.002879 0.01042] Counter Clockwise movement
          (if (< (- (Variables|Default|GetCurrentSplineKey) (* (Variables|Default|GetMovementSpeed) DeltaSeconds)) 0.0)
            (Variables|Default|SetCurrentSplineKey (+ (- (Variables|Default|GetCurrentSplineKey) (* (Variables|Default|GetMovementSpeed) DeltaSeconds)) 1.0))
            (else
              (Variables|Default|SetCurrentSplineKey (- (Variables|Default|GetCurrentSplineKey) (* (Variables|Default|GetMovementSpeed) DeltaSeconds))))))
        (:NewEnumerator3
          ;[0 0.007679 0.01042] Clear Shot movement
          (bind _bestdistance (CallFunction|FindClearShotPoint (Transformation|GetActorLocation (Game|Player|GetPlayerPawn 0))))
          (Variables|Default|SetCurrentDistance (Math|Interpolation|FInterpTo (Variables|Default|GetCurrentDistance) _bestdistance DeltaSeconds (Variables|Default|GetAimInterpolationSpeed))))))
    (:then_1
      ;[0 0.01562 0.001818] Перемещение турели
      (if (Utilities|Enum|NotEqual(Enum) (Variables|Default|GetMovementVariation) "NewEnumerator3")
        (|MoveToAndRotateForPingPong)
        (else
          (|ClearShotTurretMovement))))
    (:then_2
      ;[0.001495 0.01562 0] Поворот ShootPos стрелки в сторону игрока.
      (Transformation|SetWorldRotation (Variables|Default|GetShootPosition) (Math|Rotator|FindLookatRotation (Transformation|GetWorldLocation (Variables|Default|GetShootPosition)) (Transformation|GetActorLocation (Game|Player|GetPlayerPawn 0))) false false))))

(fn ConstructionScript
  (|CallParentFunction))

(fn FindClearShotPoint
  (params (TargetLocation :type Vector))
  (for _index (range 0 20)
    (bind _outhit (Collision|LineTraceByChannel (Spline|GetLocationatDistanceAlongSpline (Variables|Default|GetSpline) (* (/ (Math|Conversions|ToFloat(Integer) _index) 2e+01) (Variables|Default|GetSplineLength)) "World") TargetLocation "TraceTypeQuery1" false 0 "ForDuration" true "(R=1.000000,G=0.000000,B=0.000000,A=1.000000)" "(R=0.000000,G=1.000000,B=0.000000,A=1.000000)" 0.1))
    (if (not (.bBlockingHit (Collision|BreakHitResult _outhit)))
      (if (< (Math|Vector|VectorLength (- TargetLocation (Spline|GetLocationatDistanceAlongSpline (Variables|Default|GetSpline) (* (/ (Math|Conversions|ToFloat(Integer) _index) 2e+01) (Variables|Default|GetSplineLength)) "World"))) (LocalVariables|GetBestScore))
        (LocalVariables|SetBestScore (Math|Vector|VectorLength (- TargetLocation (Spline|GetLocationatDistanceAlongSpline (Variables|Default|GetSpline) (* (/ (Math|Conversions|ToFloat(Integer) _index) 2e+01) (Variables|Default|GetSplineLength)) "World"))))
        (LocalVariables|SetDistanceToShoot (* (/ (Math|Conversions|ToFloat(Integer) _index) 2e+01) (Variables|Default|GetSplineLength))))))
  (return (LocalVariables|GetDistanceToShoot)))