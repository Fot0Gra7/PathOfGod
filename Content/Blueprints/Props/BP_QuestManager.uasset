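; Quest manager actor that tracks kill quests per enemy type and signals gates when all of them are completed.
; AddQuest appends a quest struct to the ActiveQuest array; RegisterEnemyKilled increments matching quests and flags completion once required kills are reached.
; Each update refreshes the kill progress bars in the GM_Keco HUD and prints debug state.
; When every active quest is complete, it calls CallQuestCompleted on all BP_Gate actors.
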(event EventBeginPlay)

(event Collision|EventActorBeginOverlap
  (params (OtherActor :type Actor%20Object%20Reference)))

(event EventTick
  (params (DeltaSeconds :type Float%20%28single-precision%29)))

(fn ConstructionScript)

(fn AddQuest
  (params (NewQuest :type BPS%20Kill%20Quest%20Structure))
  (bind (_enemytype _requiredkills) (Utilities|Struct|BreakBPS_KillQuest NewQuest))
  (Utilities|Array|Add (Variables|Default|GetActiveQuest) NewQuest)
  (Development|PrintString (Utilities|String|Append "New Quest to kill: " (Utilities|String|EnumtoString _enemytype) " In amount of: " (Utilities|String|ToString(Integer) _requiredkills)) true true "(R=1.000000,G=1.000000,B=1.000000,A=1.000000)" 8.0))

(fn RegisterEnemyKilled
  (params (EnemyType :type E_EnemyType%20Enum :default "NewEnumerator0"))
  (for (_array_element _array_index) (Variables|Default|GetActiveQuest)
    (bind _output_get (Variables|Default|SetTempQuest _array_element))
    (if (Utilities|Enum|Equal(Enum) (.EnemyType (Utilities|Struct|BreakBPS_KillQuest _output_get)) EnemyType)
      (bind _result (Math|Integer|IncrementInt (.CurrentKills (Utilities|Struct|BreakBPS_KillQuest _output_get)))
        (:%20%20
          (if (>= _result (.RequiredKills (Utilities|Struct|BreakBPS_KillQuest _output_get)))
            (Variables|Default|SetTempQuest (Utilities|Struct|MakeBPS_KillQuest (.enemytype (Variables|Default|GetTempQuest)) (.requiredkills (Variables|Default|GetTempQuest)) (.currentkills (Variables|Default|GetTempQuest)) true))
            (Utilities|Array|SetArrayElem (Variables|Default|GetActiveQuest) _array_index (Variables|Default|GetTempQuest))
            (Utilities|FlowControl|Sequence
              (:then_0
                (for _array_element_2 (Class|PanelWidget|GetAllChildren (Variables|/Game/Widgets/W_HUD.W_HUD_C|GetKillQuestsVerticalBox (Variables|/Game/Blueprints/GM_Keco.GM_Keco_C|GetHudWidget (.AsGM%20Keco (Utilities|Casting|CastToGM_Keco (Game|GetGameMode))))))
                  (Default|UpdateKillProgressBarFill (.AsW%20Enemy%20Kill%20Quest%20Prorgess%20Bar (Utilities|Casting|CastToW_EnemyKillQuestProrgessBar _array_element_2))))
                ;[0.15 0.15 0.15 0.5] Quest State
                (Development|PrintString (Utilities|String|Append "Quest progress: " (Utilities|String|EnumtoString (.enemytype (Variables|Default|GetTempQuest))) " Kills Required: " (Utilities|String|ToString(Integer) (.requiredkills (Variables|Default|GetTempQuest))) " Current Kills: " (Utilities|String|ToString(Integer) (.currentkills (Variables|Default|GetTempQuest))) "    QuestComplition: " (Utilities|String|ToString(Boolean) (.iscompleted (Variables|Default|GetTempQuest)))) true true "(R=0.022267,G=1.000000,B=0.000000,A=1.000000)" 5.0))
              (:then_1
                (Variables|Default|SetQuestsCompleted 0)
                (for _array_element_3 (Variables|Default|GetActiveQuest)
                  (if (.IsCompleted (Utilities|Struct|BreakBPS_KillQuest _array_element_3))
                    (Math|Integer|IncrementInt (Variables|Default|GetQuestsCompleted))))
                (if (== (Variables|Default|GetQuestsCompleted) (Utilities|Array|Length (Variables|Default|GetActiveQuest)))
                  (bind _outactors (Actor|GetAllActorsOfClass "/Game/Blueprints/Props/BP_Gate.BP_Gate_C"))
                  (for _array_element_4 _outactors
                    (Default|CallQuestCompleted _array_element_4)))))
            (else
              (Variables|Default|SetTempQuest (Utilities|Struct|MakeBPS_KillQuest (.enemytype (Variables|Default|GetTempQuest)) (.requiredkills (Variables|Default|GetTempQuest)) (.currentkills (Variables|Default|GetTempQuest)) false))
              (Utilities|Array|SetArrayElem (Variables|Default|GetActiveQuest) _array_index (Variables|Default|GetTempQuest))
              (for _array_element_5 (Class|PanelWidget|GetAllChildren (Variables|/Game/Widgets/W_HUD.W_HUD_C|GetKillQuestsVerticalBox (Variables|/Game/Blueprints/GM_Keco.GM_Keco_C|GetHudWidget (.AsGM%20Keco (Utilities|Casting|CastToGM_Keco (Game|GetGameMode))))))
                (Default|UpdateKillProgressBarFill (.AsW%20Enemy%20Kill%20Quest%20Prorgess%20Bar (Utilities|Casting|CastToW_EnemyKillQuestProrgessBar _array_element_5))))
              ;[0.15 0.15 0.15 0.5] Quest State
              (Development|PrintString (Utilities|String|Append "Quest progress: " (Utilities|String|EnumtoString (.enemytype (Variables|Default|GetTempQuest))) " Kills Required: " (Utilities|String|ToString(Integer) (.requiredkills (Variables|Default|GetTempQuest))) " Current Kills: " (Utilities|String|ToString(Integer) (.currentkills (Variables|Default|GetTempQuest))) "    QuestComplition: " (Utilities|String|ToString(Boolean) (.iscompleted (Variables|Default|GetTempQuest)))) true true "(R=1.000000,G=0.912283,B=0.000000,A=1.000000)" 5.0))))))))