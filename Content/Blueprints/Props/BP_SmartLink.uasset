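; BP_SmartLink is a nav link proxy that makes BP_Pog_Enemy_BASE agents jump to the link's destination.
; When an agent reaches the link, it stops movement and clears CanMove on the blackboard and character.
; After a short delay, it launches the character on a ballistic arc computed from JumpTime, gravity and the offset to the destination.
; A fixed delay later, rather than a landing check, it restores CanMove and resumes path following.
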(event EventSmartLinkReached
  (params (Agent :type Actor%20Object%20Reference) (Destination :type Vector%20%28by%20ref%29 :default "0, 0, 0"))
  (bind _output_get (Variables|Default|SetJumpChar (.AsBP%20Pog%20Enemy%20BASE (Utilities|Casting|CastToBP_Pog_Enemy_BASE Agent))))
  (AI|Components|Blackboard|SetValueasBool (AI|GetBlackboard _output_get) (Utilities|Name|MakeLiteralName "CanMove") false)
  (Variables|/Game/Blueprints/Characters/BP_Pog_Character_BASE.BP_Pog_Character_BASE_C|SetCanMove _output_get false)
  (AI|Navigation|StopMovement (AI|GetAIController _output_get))
  (Utilities|FlowControl|Delay 0.2)
  (Character|LaunchCharacter _output_get (Math|Vector|MakeVector (.x (* (Math|Vector|Normalize (Math|Vector|MakeVector (.X (Math|Vector|BreakVector (- Destination (Transformation|GetActorLocation _output_get)))) (.Y (Math|Vector|BreakVector (- Destination (Transformation|GetActorLocation _output_get)))) 0.0)) (/ (Math|Vector|VectorLength (Math|Vector|MakeVector (.X (Math|Vector|BreakVector (- Destination (Transformation|GetActorLocation _output_get)))) (.Y (Math|Vector|BreakVector (- Destination (Transformation|GetActorLocation _output_get)))) 0.0)) (Variables|Default|GetJumpTime)))) (.y (* (Math|Vector|Normalize (Math|Vector|MakeVector (.X (Math|Vector|BreakVector (- Destination (Transformation|GetActorLocation _output_get)))) (.Y (Math|Vector|BreakVector (- Destination (Transformation|GetActorLocation _output_get)))) 0.0)) (/ (Math|Vector|VectorLength (Math|Vector|MakeVector (.X (Math|Vector|BreakVector (- Destination (Transformation|GetActorLocation _output_get)))) (.Y (Math|Vector|BreakVector (- Destination (Transformation|GetActorLocation _output_get)))) 0.0)) (Variables|Default|GetJumpTime)))) (/ (+ (* (* (Math|Float|Absolute(Float) (Components|Movement|GetGravityZ (Variables|/Script/Engine.Character|GetCharacterMovement _output_get))) 0.5) (Math|Float|Square (Variables|Default|GetJumpTime))) (- (.Z (Math|Vector|BreakVector Destination)) (.Z (Math|Vector|BreakVector (Transformation|GetActorLocation _output_get))))) (Variables|Default|GetJumpTime))) true true)
  (Utilities|FlowControl|Delay 1.0)
  (AI|Components|Blackboard|SetValueasBool (AI|GetBlackboard _output_get) (Utilities|Name|MakeLiteralName "CanMove") true)
  (Variables|/Game/Blueprints/Characters/BP_Pog_Character_BASE.BP_Pog_Character_BASE_C|SetCanMove _output_get true)
  (Class|NavLinkProxy|ResumePathFollowing _output_get))

(fn ConstructionScript)