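; Base trap actor for a Paper2D prop that, when destructible, loses durability to Pog character attack hitboxes and is destroyed at zero.
; Each hit applies damage and triggers hit stop on the attacker; a DoOnce gate limits durability loss until the reaction finishes.
; Surviving hits briefly deactivate the trap, freeze it via custom time dilation, and shake the flipbook on a looping FlipFlop timer before restoring its position.
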(event OnComponentBeginOverlap(TrapHitbox)
  (params (OverlappedComponent :type Primitive%20Component%20Object%20Reference) (OtherActor :type Actor%20Object%20Reference) (OtherComp :type Primitive%20Component%20Object%20Reference) (OtherBodyIndex :type Integer) (bFromSweep :type Boolean) (SweepResult :type Hit%20Result%20Structure%20%28by%20ref%29))
  (if (Variables|Default|GetIsDestructible)
    (bind _asbp_pog_character_base (Utilities|Casting|CastToBP_Pog_Character_BASE OtherActor))
    (if (Components|ComponentHasTag OtherComp "AttackHitbox")
      (Game|Damage|ApplyDamage self 1.0 0 _asbp_pog_character_base)
      (Default|HitStopSequence _asbp_pog_character_base 0.2)
      (Utilities|FlowControl|DoOnce false
        (:Completed
          (Math|Float|DecrementFloat (Variables|Default|GetCurrentDurability)
            (:%20%20
              (if (> (Variables|Default|GetCurrentDurability) 0.0)
                (CallFunction|TrapHitStop)
                (Variables|Default|SetIsActive false)
                (bind _returnvalue (Utilities|Time|SetTimerbyEvent (delegate Custom|ShakeSprite) 0.05 true))
                (bind _output_get (Variables|Default|SetSpriteShakeTimer _returnvalue))
                (Utilities|FlowControl|RetriggerableDelay 0.2)
                (Utilities|Time|ClearandInvalidateTimerbyHandle _output_get)
                (Transformation|SetRelativeLocation (Variables|Default|GetPaperFlipbook) (Variables|Default|GetSpriteBaseLocation) false false)
                (Variables|Default|SetIsActive true)
                (CallFunction|ResetDamageRecieve)
                (else
                  (Actor|DestroyActor))))))))))

(event Custom|TrapHitStop
  (Variables|Default|SetCustomTimeDilation 0.0)
  (Utilities|FlowControl|RetriggerableDelay 0.2)
  (Variables|Default|SetCustomTimeDilation 1.0))

(event Custom|ResetDamageRecieve
  (Utilities|FlowControl|DoOnce false) ; enters at Reset
)

(event Custom|ShakeSprite
  (bind _spritebaselocation (Variables|Default|GetSpriteBaseLocation))
  (bind _isa (Utilities|FlowControl|FlipFlop)
    (:A
      _)
    (:B
      _))
  (Transformation|SetRelativeLocation (Variables|Default|GetPaperFlipbook) (Math|Vector|MakeVector (+ (.x _spritebaselocation) (select _isa (Variables|Default|GetSpriteShakeDistance) (* (Variables|Default|GetSpriteShakeDistance) -1.0))) (.y _spritebaselocation) (.z _spritebaselocation)) false false))

(event EventBeginPlay
  (Variables|Default|SetCurrentDurability (Variables|Default|GetMaxDurability))
  (Variables|Default|SetSpriteBaseLocation (Variables|/Script/Engine.SceneComponent|GetRelativeLocation (Variables|Default|GetPaperFlipbook))))

(event Collision|EventActorBeginOverlap
  (params (OtherActor :type Actor%20Object%20Reference)))

(event EventTick
  (params (DeltaSeconds :type Float%20%28single-precision%29)))

(fn ConstructionScript)