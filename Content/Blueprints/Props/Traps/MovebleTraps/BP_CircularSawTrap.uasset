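; BP_CircularSawTrap is a spinning saw trap that damages the player on contact.
; Tick rotates the Paper2D flipbook around its pitch axis at RotationSpeed, scaled by delta time.
; Overlapping DamageTrigger applies damage to BP_Player_Keco if the player is not invincible and CanDamage is set.
; It then blocks further hits until a timer matching the player's InvincibilityDuration resets CanDamage.
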(event OnComponentBeginOverlap(DamageTrigger)
  (params (OverlappedComponent :type Primitive%20Component%20Object%20Reference) (OtherActor :type Actor%20Object%20Reference) (OtherComp :type Primitive%20Component%20Object%20Reference) (OtherBodyIndex :type Integer) (bFromSweep :type Boolean) (SweepResult :type Hit%20Result%20Structure%20%28by%20ref%29))
  (bind _asbp_player_keco (Utilities|Casting|CastToBP_Player_Keco OtherActor))
  (if (and (not (Variables|/Game/Blueprints/Characters/BP_Pog_Character_BASE.BP_Pog_Character_BASE_C|GetIsInvincible _asbp_player_keco)) (Variables|Default|GetCanDamage))
    (Variables|Default|SetCanDamage false)
    (Game|Damage|ApplyDamage _asbp_player_keco 1.0 0 self)
    (Utilities|Time|SetTimerbyEvent (delegate Custom|ResetDamage) (Variables|/Game/Blueprints/Characters/Keco/BP_Player_Keco.BP_Player_Keco_C|GetInvincibilityDuration _asbp_player_keco))))

(event Custom|ResetDamage
  (Variables|Default|SetCanDamage true))

(event EventBeginPlay
  (|CallParentFunction) ; This node is disabled and will not be called.\nDrag off pins to build functionality.
)

(event Collision|EventActorBeginOverlap
  (params (OtherActor :type Actor%20Object%20Reference))
  (|CallParentFunction OtherActor) ; This node is disabled and will not be called.\nDrag off pins to build functionality.
)

(event EventTick
  (params (DeltaSeconds :type Float%20%28single-precision%29))
  (|CallParentFunction DeltaSeconds)
  (Transformation|AddLocalRotation (Variables|Default|GetPaperFlipbook) (Math|Rotator|MakeRotator 0.0 (* DeltaSeconds (Variables|Default|GetRotationSpeed)) 0.0) false false))

(fn ConstructionScript
  (|CallParentFunction))