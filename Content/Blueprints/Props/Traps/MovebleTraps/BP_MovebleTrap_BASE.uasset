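; Base moving trap that travels along a spline and can act as a projectile turret firing fireballs at the player.
; Tick moves TrapRoot in ping-pong, looping or Clear Shot mode, which samples the spline with line traces to approach the nearest unobstructed point to the player.
; Turrets aim with optional quaternion smoothing, fire and reload on timers, restart the fire timer when damaged, and link to an ammo widget.
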(event Custom|Shoot
  (if (Variables|Default|GetIsActive)
    (if (not (Variables|Projectiles|GetIsReloading))
      (if (> (Variables|Projectiles|GetCurrentAmmo) 0)
        (CallFunction|ShootProjectile)
        (Math|Integer|DecrementInt (Variables|Projectiles|GetCurrentAmmo))
        (else
          (CallFunction|Reload))))))

(event Custom|ShootStart
  (if (Variables|Default|GetProjectileBasedTurret)
    (bind _returnvalue (Utilities|Time|SetTimerbyEvent (delegate Custom|Shoot) (Variables|Projectiles|GetFireRate) true))
    (Variables|Projectiles|SetShootTimer _returnvalue)))

(event Custom|Reload
  (Utilities|Time|ClearandInvalidateTimerbyHandle (Variables|Projectiles|GetShootTimer))
  (Variables|Projectiles|SetIsReloading true)
  (Utilities|FlowControl|Delay (Variables|Projectiles|GetReloadTime))
  (Variables|Projectiles|SetCurrentAmmo (Variables|Projectiles|GetMaxAmmo))
  (Variables|Projectiles|SetIsReloading false)
  (CallFunction|ShootStart))

(event EventBeginPlay
  (|CallParentFunction)
  (Variables|Default|SetSplineLength (Spline|GetSplineLength (Variables|Default|GetSpline)))
  (Utilities|FlowControl|Sequence
    (:then_1
      ;[0.000599 0.02083 0 1 16] Можно добавить Delay, чтобы начинала перезаряжаться не сразу
      (CallFunction|ShootStart))
    (:then_2
      ;[0.001193 0.02083 0] Привязка турели к виджету, чтобы он получал её данные
      (bind _asw_turret_ammo (Utilities|Casting|CastToW_TurretAmmo (UserInterface|GetUserWidgetObject (Variables|Default|GetTurretWidget))))
      (Default|SetOwningTurret _asw_turret_ammo self))))

(event Collision|EventActorBeginOverlap
  (params (OtherActor :type Actor%20Object%20Reference))
  (|CallParentFunction OtherActor) ; This node is disabled and will not be called.\nDrag off pins to build functionality.
)

(event EventTick
  (params (DeltaSeconds :type Float%20%28single-precision%29))
  (bind _returnvalue (Game|Player|GetPlayerPawn 0))
  (bind _shootposition (Variables|Default|GetShootPosition))
  (bind _returnvalue_2 (Transformation|GetActorLocation _returnvalue))
  (bind _returnvalue_3 (Transformation|GetWorldLocation _shootposition))
  (bind _returnvalue_4 (- _returnvalue_2 _returnvalue_3))
  (bind _returnvalue_5 (Math|Vector|Normalize _returnvalue_4))
  (|CallParentFunction DeltaSeconds)
  (if (Variables|Default|GetIsActive)
    (Utilities|FlowControl|Sequence
      (:then_0
        (switch Utilities|FlowControl|Switch|SwitchonE_Trap_Movement_Variation (Variables|Movement|GetMovementVariation)
          (:NewEnumerator0
            ;[0 0.003766 0.01042] Ping Pong movement
            (if (Variables|Movement|GetIsMovingForward)
              (if (>= (+ (Variables|Movement|GetCurrentSplineKey) (* (Variables|Movement|GetMovementSpeed) DeltaSeconds)) 1.0)
                (Variables|Movement|SetCurrentSplineKey 1.0)
                (Variables|Movement|SetIsMovingForward false)
                (else
                  (Variables|Movement|SetCurrentSplineKey (+ (Variables|Movement|GetCurrentSplineKey) (* (Variables|Movement|GetMovementSpeed) DeltaSeconds)))))
              (elif (<= (- (Variables|Movement|GetCurrentSplineKey) (* (Variables|Movement|GetMovementSpeed) DeltaSeconds)) 0.0)
                (Variables|Movement|SetCurrentSplineKey 0.0)
                (Variables|Movement|SetIsMovingForward true)
                (else
                  (Variables|Movement|SetCurrentSplineKey (- (Variables|Movement|GetCurrentSplineKey) (* (Variables|Movement|GetMovementSpeed) DeltaSeconds)))))))
          (:NewEnumerator1
            ;[0 0.01953 0.02083] Clockwise movement
            (if (> (+ (Variables|Movement|GetCurrentSplineKey) (* (Variables|Movement|GetMovementSpeed) DeltaSeconds)) 1.0)
              (Variables|Movement|SetCurrentSplineKey (- (+ (Variables|Movement|GetCurrentSplineKey) (* (Variables|Movement|GetMovementSpeed) DeltaSeconds)) 1.0))
              (else
                (Variables|Movement|SetCurrentSplineKey (+ (Variables|Movement|GetCurrentSplineKey) (* (Variables|Movement|GetMovementSpeed) DeltaSeconds))))))
          (:NewEnumerator2
            ;[0 0.002879 0.01042] Counter Clockwise movement
            (if (< (- (Variables|Movement|GetCurrentSplineKey) (* (Variables|Movement|GetMovementSpeed) DeltaSeconds)) 0.0)
              (Variables|Movement|SetCurrentSplineKey (+ (- (Variables|Movement|GetCurrentSplineKey) (* (Variables|Movement|GetMovementSpeed) DeltaSeconds)) 1.0))
              (else
                (Variables|Movement|SetCurrentSplineKey (- (Variables|Movement|GetCurrentSplineKey) (* (Variables|Movement|GetMovementSpeed) DeltaSeconds))))))
          (:NewEnumerator3
            ;[0 0.007679 0.01042] Clear Shot movement
            (bind _bestdistance (CallFunction|FindClearShotPoint (Transformation|GetActorLocation (Game|Player|GetPlayerPawn 0))))
            (Variables|ClearShot|SetCurrentDistance (Math|Interpolation|FInterpTo (Variables|ClearShot|GetCurrentDistance) _bestdistance DeltaSeconds (Variables|ClearShot|GetAimInterpolationSpeed))))))
      (:then_1
        ;[0 0.01562 0.001818] Перемещение турели
        (if (Utilities|Enum|NotEqual(Enum) (Variables|Movement|GetMovementVariation) "NewEnumerator3")
          (|MoveToAndRotateForPingPong)
          (else
            (|ClearShotTurretMovement))))
      (:then_2
        ;[0.001495 0.01562 0] Поворот ShootPos стрелки в сторону игрока.
        (if (Variables|Default|GetProjectileBasedTurret)
          (Transformation|SetWorldRotation (Variables|Default|GetShootPosition) (select (Variables|Default|GetSmoothRotation) (Class|KismetMathLibrary|QuatRotator (Class|KismetMathLibrary|QuatSlerp (Math|Conversions|ToQuaternion(Rotator) (Transformation|GetWorldRotation (Variables|Default|GetShootPosition))) (Math|Conversions|ToQuaternion(Rotator) (Math|Rotator|MakeRotator 0.0 (Math|Trig|RadiansToDegrees (Math|Trig|Atan2(Radians) (.z _returnvalue_5) (.x _returnvalue_5))) 0.0)) (* DeltaSeconds (Variables|Default|GetSmoothRotationSpeed)))) (Math|Rotator|FindLookatRotation (Transformation|GetWorldLocation (Variables|Default|GetShootPosition)) (Transformation|GetActorLocation (Game|Player|GetPlayerPawn 0)))) false false))))))

(event Game|Damage|EventAnyDamage
  (params (Damage :type Float%20%28single-precision%29) (DamageType :type Damage%20Type%20Object%20Reference) (InstigatedBy :type Controller%20Object%20Reference) (DamageCauser :type Actor%20Object%20Reference))
  (|CallParentFunction Damage DamageType InstigatedBy DamageCauser)
  (if (Variables|Default|GetProjectileBasedTurret)
    (Utilities|Time|ClearandInvalidateTimerbyHandle (Variables|Projectiles|GetShootTimer))
    (CallFunction|ShootStart)))

(event Input|KeyboardEvents|1
  (params (Key :type Key%20Structure :default "None"))
  ;[0.06771 0 0.000874] Удалить потом
  (:Pressed
    (if (Variables|Default|GetProjectileBasedTurret)
      (CallFunction|ShootProjectile))))

(fn ConstructionScript
  (|CallParentFunction))

(fn FindClearShotPoint
  (params (TargetLocation :type Vector))
  (for _index (range 0 20)
    (bind _outhit (Collision|LineTraceByChannel (Spline|GetLocationatDistanceAlongSpline (Variables|Default|GetSpline) (* (/ (Math|Conversions|ToFloat(Integer) _index) 2e+01) (Variables|Default|GetSplineLength)) "World") TargetLocation "TraceTypeQuery1" false 0 "None" true "(R=1.000000,G=0.000000,B=0.000000,A=1.000000)" "(R=0.000000,G=1.000000,B=0.000000,A=1.000000)" 0.1))
    (if (not (.bBlockingHit (Collision|BreakHitResult _outhit)))
      (if (< (Math|Vector|VectorLength (- TargetLocation (Spline|GetLocationatDistanceAlongSpline (Variables|Default|GetSpline) (* (/ (Math|Conversions|ToFloat(Integer) _index) 2e+01) (Variables|Default|GetSplineLength)) "World"))) (LocalVariables|GetBestScore))
        (LocalVariables|SetBestScore (Math|Vector|VectorLength (- TargetLocation (Spline|GetLocationatDistanceAlongSpline (Variables|Default|GetSpline) (* (/ (Math|Conversions|ToFloat(Integer) _index) 2e+01) (Variables|Default|GetSplineLength)) "World"))))
        (LocalVariables|SetDistanceToShoot (* (/ (Math|Conversions|ToFloat(Integer) _index) 2e+01) (Variables|Default|GetSplineLength))))))
  (return (LocalVariables|GetDistanceToShoot)))

(fn ShootProjectile
  (bind _shootposition (Variables|Default|GetShootPosition))
  (bind _returnvalue (Transformation|GetWorldTransform _shootposition))
  (Game|SpawnActorfromClass "/Game/Blueprints/Projectiles/BP_Pog_EnemyFireball.BP_Pog_EnemyFireball_C" (Math|Transform|MakeTransform (.location _returnvalue) (.rotation _returnvalue) "1.000000,1.000000,1.000000") "AlwaysSpawn" "MultiplyWithRoot" self 0))