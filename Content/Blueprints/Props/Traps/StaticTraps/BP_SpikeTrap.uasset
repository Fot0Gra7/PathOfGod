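; BP_SpikeTrap is a static spike trap with a Paper2D flipbook that rises from below to hurt the player when triggered.
; A trigger box overlap by the player, while the trap is active, starts a delayed timeline that lerps the spikes up, then reverses it after a pause.
; A separate damage collision applies damage to non-invincible players, then blocks further hits until a timer matching the player's invincibility duration re-enables it.
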(event OnComponentBeginOverlap(TrapTriggerBox)
  (params (OverlappedComponent :type Primitive%20Component%20Object%20Reference) (OtherActor :type Actor%20Object%20Reference) (OtherComp :type Primitive%20Component%20Object%20Reference) (OtherBodyIndex :type Integer) (bFromSweep :type Boolean) (SweepResult :type Hit%20Result%20Structure%20%28by%20ref%29))
  (Utilities|Casting|CastToBP_Player_Keco OtherActor)
  (if (and (Variables|Default|GetIsActive) (not (Variables|Default|GetIsTriggered)))
    (Variables|Default|SetIsTriggered true)
    (Utilities|FlowControl|Delay 1.0)
    (CallFunction|ActivateSpikes)
    (Utilities|FlowControl|Delay 2.0)
    (CallFunction|ResetSpikes)))

(event OnComponentBeginOverlap(DamageCollision)
  (params (OverlappedComponent :type Primitive%20Component%20Object%20Reference) (OtherActor :type Actor%20Object%20Reference) (OtherComp :type Primitive%20Component%20Object%20Reference) (OtherBodyIndex :type Integer) (bFromSweep :type Boolean) (SweepResult :type Hit%20Result%20Structure%20%28by%20ref%29))
  (bind _asbp_player_keco (Utilities|Casting|CastToBP_Player_Keco OtherActor))
  (if (and (not (Variables|/Game/Blueprints/Characters/BP_Pog_Character_BASE.BP_Pog_Character_BASE_C|GetIsInvincible _asbp_player_keco)) (Variables|Default|GetCanDamage))
    (Variables|Default|SetCanDamage false)
    (Game|Damage|ApplyDamage _asbp_player_keco 1.0 0 self)
    (Utilities|Time|SetTimerbyEvent (delegate Custom|ResetDamage) (Variables|/Game/Blueprints/Characters/Keco/BP_Player_Keco.BP_Player_Keco_C|GetInvincibilityDuration _asbp_player_keco))))

(event Custom|ActivateSpikes
  (bind _traplocation (Timeline|SpikeMovementTimeline Play)
    (:Update
      (Transformation|SetRelativeLocation (Variables|Default|GetPaperFlipbook) (Math|Vector|Lerp(Vector) "0.000000,0.000000,-70.000000" "0, 0, 0" _traplocation) false false))))

(event Custom|ResetSpikes
  (Variables|Default|SetIsTriggered false)
  (bind _traplocation (Timeline|SpikeMovementTimeline Reverse)
    (:Update
      (Transformation|SetRelativeLocation (Variables|Default|GetPaperFlipbook) (Math|Vector|Lerp(Vector) "0.000000,0.000000,-70.000000" "0, 0, 0" _traplocation) false false))))

(event Custom|ResetDamage
  (Variables|Default|SetCanDamage true))

(event EventBeginPlay
  (|CallParentFunction) ; This node is disabled and will not be called.\nDrag off pins to build functionality.
)

(event Collision|EventActorBeginOverlap
  (params (OtherActor :type Actor%20Object%20Reference))
  (|CallParentFunction OtherActor) ; This node is disabled and will not be called.\nDrag off pins to build functionality.
)

(event EventTick
  (params (DeltaSeconds :type Float%20%28single-precision%29))
  (|CallParentFunction DeltaSeconds) ; This node is disabled and will not be called.\nDrag off pins to build functionality.
)

(fn ConstructionScript
  (|CallParentFunction))