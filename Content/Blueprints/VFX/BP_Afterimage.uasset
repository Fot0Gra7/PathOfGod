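; BP_Afterimage is a visual effect actor that leaves a fading sprite copy of its owner character's current pose.
; On BeginPlay it copies the owner's current flipbook frame onto its PaperSprite and creates a dynamic material instance.
; A Dissolve timeline, with play rate scaled by the inverse of DissolveTime, drives the material's Alpha parameter and destroys the actor when finished.
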(event EventBeginPlay
  (bind _ownercharacter (Variables|Default|GetOwnerCharacter))
  (bind _papersprite (Variables|Default|GetPaperSprite))
  (bind _sprite (Variables|/Script/Paper2D.PaperCharacter|GetSprite _ownercharacter))
  (bind _returnvalue (Rendering|Material|CreateDynamicMaterialInstance _papersprite 0 (Rendering|Material|GetMaterial _papersprite 0) "None" :!class /Script/Engine.PrimitiveComponent))
  (Rendering|Components|Sprite|SetSprite (Variables|Default|GetPaperSprite) (Class|PaperFlipbook|GetSpriteatFrame (Class|PaperFlipbookComponent|GetFlipbook _sprite) (Class|PaperFlipbookComponent|GetPlaybackPositioninFrames _sprite)))
  (Components|Timeline|SetPlayRate (Variables|DONOTEDIT|GetDissolve) (/ 1.0 (Variables|Default|GetDissolveTime)))
  (bind _alphadissolvetrack (Timeline|Dissolve PlayFromStart)
    (:Update
      (Rendering|Material|SetScalarParameterValue _returnvalue "Alpha" _alphadissolvetrack :!class /Script/Engine.MaterialInstanceDynamic))
    (:Finished
      (Actor|DestroyActor))))

(fn ConstructionScript)